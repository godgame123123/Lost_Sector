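; BP_LootBox is an interactable loot container actor that opens a looting screen for the player.
; Interact accepts only a PlayerCharacter, creates WB_looting linked to the box, applies GetUIItems' result, then switches to UI-only input with a cursor.
; GetUIItems loops over ChestItems with an empty body, leaving its conversion code disconnected, so ResultItems is never filled here.
; ConvertToUIData maps item stacks to grid-sized UI data but is not called here.
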(event EventBeginPlay)

(event Collision|EventActorBeginOverlap
  (params (OtherActor :type Actor%20Object%20Reference)))

(event EventTick
  (params (DeltaSeconds :type Float%20%28single-precision%29)))

(event EventInteract
  (params (ByWho :type Character%20Object%20Reference))
  (bind _returnvalue (Game|GetPlayerController 0))
  (Utilities|Casting|CastToPlayerCharacter ByWho)
  (bind _returnvalue_2 (UserInterface|CreateWidget "/Game/Team_Folder/LHJ/UI/WB_looting.WB_looting_C" (Game|GetPlayerController 0) 0))
  (bind _output_get (Variables|Default|SetLootUI _returnvalue_2))
  (Variables|/Game/Team_Folder/LHJ/UI/WB_looting.WB_looting_C|SetContainerRef _returnvalue_2 self)
  (bind _itemsui (CallFunction|GetUIItems))
  (Default|ApplyItems _output_get _itemsui)
  (Development|PrintString "opne chest")
  (UserInterface|Viewport|AddtoViewport _output_get 100)
  (Input|SetInputModeUIOnly _returnvalue _output_get "DoNotLock" false)
  (Variables|/Script/Engine.PlayerController|SetbShowMouseCursor _returnvalue true))

(fn ConstructionScript)

(fn ConverttoUIData
  (params (ItemStack :type Item%20Stack%20Structure))
  (bind _item (Utilities|Struct|BreakItemStack ItemStack))
  (return (Utilities|Struct|MakeST_ItemData 0 0 (Variables|/Script/LostSector.ItemDataBase|GetGridWidth _item) (Variables|/Script/LostSector.ItemDataBase|GetGridHeight _item) (Variables|/Script/LostSector.ItemDataBase|GetIcon _item) (Variables|/Script/LostSector.ItemDataBase|GetDisplayName _item))))

(fn GetUIItems
  (for _array_element (Variables|Default|GetChestItems)
    _)
  (return (LocalVariables|GetResultItems)))