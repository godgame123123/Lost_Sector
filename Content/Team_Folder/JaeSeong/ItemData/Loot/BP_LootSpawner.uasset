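; BP_LootSpawner is a placeable spawner that creates one item pickup at its own transform on BeginPlay, on the authority only.
; GetLoot supplies the pickup's item stack, with a random count between the chosen LootTable entry's min and max.
; Selection is built as a cumulative-weight roll, but RandomValue is set to zero and the random float node is unused, so the first entry normally wins.
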(event EventBeginPlay
  (if (Ability|HasAuthority)
    (bind _returnvalue (CallFunction|GetLoot))
    (bind _returnvalue_2 (Game|SpawnActorfromClass "/Script/LostSector.ItemPickup" (Transformation|GetActorTransform) "AlwaysSpawn" "MultiplyWithRoot" 0 0))
    (Development|PrintString "spawn")
    (Variables|/Script/LostSector.ItemPickup|SetStack _returnvalue_2 (Utilities|Struct|MakeItemStack (.Item (Utilities|Struct|BreakItemStack _returnvalue)) "None" (.Count (Utilities|Struct|BreakItemStack _returnvalue))))))

(event Collision|EventActorBeginOverlap
  (params (OtherActor :type Actor%20Object%20Reference)))

(event EventTick
  (params (DeltaSeconds :type Float%20%28single-precision%29)))

(fn ConstructionScript)

(fn GetLoot
  (for _array_element (Variables|/Game/Team_Folder/JaeSeong/ItemData/Loot/DA_LootTableBase.DA_LootTableBase_C|GetLoots (Variables|Default|GetLootTable))
    (LocalVariables|SetTotalWeight (+ (LocalVariables|GetTotalWeight) (.Weight (Utilities|Struct|BreakST_DropItem _array_element)))))
  (Utilities|FlowControl|Sequence
    (:then_0
      (bind _output_get (LocalVariables|SetRandomValue 0.0)))
    (:then_1
      (for _array_element_2 (Variables|/Game/Team_Folder/JaeSeong/ItemData/Loot/DA_LootTableBase.DA_LootTableBase_C|GetLoots (Variables|Default|GetLootTable))
        (bind _output_get_2 (LocalVariables|SetAccWeight (+ (LocalVariables|GetAccWeight) (.Weight (Utilities|Struct|BreakST_DropItem _array_element_2)))))
        (if (<= (LocalVariables|GetRandomValue) _output_get_2)
          (bind _output_get_3 (LocalVariables|SetSelectedLoot _array_element_2))
          (return (Utilities|Struct|MakeItemStack (.Item (Utilities|Struct|BreakST_DropItem _output_get_3)) "None" (Math|Random|RandomIntegerinRange (.MinCount (Utilities|Struct|BreakST_DropItem _output_get_3)) (.MaxCount (Utilities|Struct|BreakST_DropItem _output_get_3))))))))))